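; Interaction prompt actor that lets the player collect items from nearby Dispenser actors.
; Each tick it finds the closest enabled Dispenser within range of the player, moves itself onto it and shows its prompt, or hides far below the world when none is near.
; The text turns to face the IsometricCharacter's top-down camera, and pressing E calls GiveCollectible on that Dispenser and plays a swipe sound.
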(event EventBeginPlay
  ;[1 1 1] enable input
  (Input|EnableInput (Game|GetPlayerController 0)))

(event EventTick
  (params (DeltaSeconds :type Float%20%28single-precision%29))
  ;[1 1 1] rotate text towards camera
  (bind _asisometric_character (Utilities|Casting|CastToIsometricCharacter (Game|Player|GetPlayerPawn 0)))
  (Transformation|SetWorldRotation (Variables|Default|Gettext_root) (Math|Rotator|FindLookatRotation (Transformation|GetWorldLocation (Variables|Default|Gettext_root)) (Transformation|GetWorldLocation (Variables|/Game/Blueprints/IsometricCharacter.IsometricCharacter_C|GetTop-Down%20Camera _asisometric_character))) false false)
  (Variables|Default|Setclosest_distance 5e+02)
  (Variables|Default|Sethas_closest false)
  (bind _outactors (Actor|GetAllActorsOfClass "/Game/Blueprints/dispensers/dispenser.dispenser_C"))
  (for _array_element _outactors
    (if (Math|Boolean|ANDBoolean (< (Math|Vector|VectorLength (- (Transformation|GetActorLocation (Game|Player|GetPlayerPawn 0)) (Transformation|GetActorLocation _array_element))) (Variables|Default|Getclosest_distance)) (< (Math|Vector|VectorLength (- (Transformation|GetActorLocation (Game|Player|GetPlayerPawn 0)) (Transformation|GetActorLocation _array_element))) 2e+02) (Variables|/Game/Blueprints/dispensers/dispenser.dispenser_C|Getenabled _array_element))
      (Variables|Default|Setclosest_distance (Math|Vector|VectorLength (- (Transformation|GetActorLocation (Game|Player|GetPlayerPawn 0)) (Transformation|GetActorLocation _array_element))))
      (Variables|Default|Setclosest_dispenser _array_element)
      (Variables|Default|Sethas_closest true)))
  (if (Variables|Default|Gethas_closest)
    (Transformation|SetActorLocation self (Transformation|GetActorLocation (Variables|Default|Getclosest_dispenser)) false true)
    (Rendering|Components|TextRender|SetText (Variables|Default|Gettext) (Utilities|Text|ToText(String) (Utilities|String|Append "[E] " (Variables|/Game/Blueprints/dispensers/dispenser.dispenser_C|Getprompt (Variables|Default|Getclosest_dispenser)))))
    (else
      (Transformation|SetActorLocation "0, 0,-1000000.000000" false true))))

(event Input|KeyboardEvents|E
  (params (Key :type Key%20Structure :default "AnyKey"))
  (:Pressed
    (if (Variables|Default|Gethas_closest)
      (Default|GiveCollectible (Variables|Default|Getclosest_dispenser))
      (Audio|PlaySound2D "/Game/Sound/swipe_item.swipe_item"))))

(fn ConstructionScript)