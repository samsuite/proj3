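; Placer tool that lets the player use an ink bomb on a container or set one on the ground.
; While selected, Tick flags a hovered container near the player as the target, swapping the placement cubes for a reticle on it.
; Left click uses the bomb on that target, or spawns a non-projectile bomb at a valid hit point.
; Either successful action notifies IsometricPlayerController that the tool was used.
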(event EventBeginPlay
  (|CallParentFunction))

(event EventTick
  (params (DeltaSeconds :type Float%20%28single-precision%29))
  (bind _reticle (Variables|Default|Getreticle))
  ;[1 1 1] if the mouse is over a container
  (|CallParentFunction 0.0)
  (if (Variables|Default|Getselected)
    (if (and (Utilities|ClassIsChildOf (Utilities|GetClass (Variables|Default|Gethovered_object)) "/Game/Blueprints/container.container_C") (< (Math|Vector|VectorLength (- (- (Transformation|GetActorLocation (Game|Player|GetPlayerPawn 0)) "0, 0,98.000000") (Variables|Default|Gethit_point))) 2.5e+02))
      (Rendering|SetVisibility (Variables|Default|Getgoodcube) false true)
      (Transformation|SetWorldLocation _reticle (Transformation|GetActorLocation (Variables|Default|Gethovered_object)) false true)
      (Rendering|SetVisibility _reticle true false)
      (Variables|Default|Sethas_target true)
      (else
        (Rendering|SetVisibility (Variables|Default|Getreticle) false true)
        (Variables|Default|Sethas_target false)))))

(event Input|MouseEvents|LeftMouseButton
  (params (Key :type Key%20Structure :default "AnyKey"))
  (:Pressed
    (if (Variables|Default|Gethas_target)
      ;[1 1 1] if we have a target, use a bomb on it !
      (bind _ascontainer (Utilities|Casting|CastTocontainer (Variables|Default|Gethovered_object)))
      (Default|UseItemon _ascontainer "/Game/Blueprints/ink_bomb.ink_bomb_C")
      ;[1 1 1] set as used
      (bind _asisometric_player_controller (Utilities|Casting|CastToIsometricPlayerController (Game|GetPlayerController 0) :!label _label))
      (Default|UsedTool _asisometric_player_controller)
      (else
        ;[1 1 1] otherwise just place a bomb on the ground
        (if (Variables|Default|Getvalid_position)
          (bind _returnvalue (Game|SpawnActorfromClass "/Game/Blueprints/ink_bomb.ink_bomb_C" (Math|Conversions|ToTransform(Vector) (Variables|Default|Gethit_point)) "Undefined" 0 0))
          (Transformation|SetActorRotation _returnvalue (Variables|Default|Getrotation))
          (Variables|/Game/Blueprints/holdable.holdable_C|Setis_projectile _returnvalue false)
          (Default|Init _returnvalue)
          (goto _label))))))

(fn ConstructionScript
  (|CallParentFunction))