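; Security camera actor that rotates, optionally ping-ponging between yaw limits, and ends the game shortly after spotting the player.
; Each tick it detects the player by range, spotlight cone angle and a line trace that ignores glass walls.
; Spotting turns the light red and shows a camera-facing countdown that calls GameOver on the IsometricPlayerController when it expires.
; Disable and Reset manage its state; the construction script draws debug sweep limits.
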(event EventTick
  (params (DeltaSeconds :type Float%20%28single-precision%29))
  (bind _returnvalue (Game|Player|GetPlayerPawn 0))
  (bind _self self)
  (bind _self_2 self)
  (bind _self_3 self)
  (bind _self_4 self)
  (bind _timer (Variables|Default|Gettimer))
  (bind _defaultsceneroot (Variables|Default|GetDefaultSceneRoot))
  (bind _returnvalue_2 (Transformation|GetActorRotation _self))
  (bind _returnvalue_3 (Transformation|GetActorRotation _self_2))
  (bind _returnvalue_4 (Transformation|GetWorldLocation _defaultsceneroot))
  (bind _returnvalue_5 (Transformation|GetActorRotation _self_3))
  (bind _returnvalue_6 (Transformation|GetActorRotation _self_4))
  (bind _returnvalue_7 (Transformation|GetActorLocation _returnvalue))
  (bind (_roll _pitch _yaw) (Math|Rotator|BreakRotator _returnvalue_2))
  (bind (_roll_2 _pitch_2 _yaw_2) (Math|Rotator|BreakRotator _returnvalue_3))
  (bind (_roll_3 _pitch_3 _yaw_3) (Math|Rotator|BreakRotator _returnvalue_5))
  (bind _yaw_4 (Math|Rotator|BreakRotator _returnvalue_6))
  (bind _returnvalue_8 (- _returnvalue_7 "0.000000, 0,50.000000"))
  (bind _returnvalue_9 (+ _yaw_4 3.6e+02))
  (bind _returnvalue_10 (Math|Float|%(Float) _returnvalue_9 3.6e+02))
  ;[1 1 1] make sure camera is on
  (if (Variables|Default|Getwatching)
    (if (Variables|Default|Getrotating)
      (if (Variables|Default|Getpingpong)
        (if (Variables|Default|Getis_counterclockwise)
          (Transformation|SetActorRotation (Math|Rotator|MakeRotator _roll_2 _pitch_2 (+ _yaw_2 (* (Variables|Default|Getrot_speed) DeltaSeconds))))
          (else
            (Transformation|SetActorRotation (Math|Rotator|MakeRotator _roll_3 _pitch_3 (+ _yaw_3 (* (* (Variables|Default|Getrot_speed) DeltaSeconds) -1.0))))))
        (Development|PrintString (Utilities|String|ToString(Float) _returnvalue_10) true true "(R=0.000000,G=0.660000,B=1.000000,A=1.000000)" 0.0)
        (if (>= _returnvalue_10 (Variables|Default|Getmax_angle))
          (Variables|Default|Setis_counterclockwise false))
        (if (<= (Math|Float|%(Float) (+ (.Yaw (Math|Rotator|BreakRotator (Transformation|GetActorRotation self))) 3.6e+02) 3.6e+02) (Variables|Default|Getmin_angle))
          (Variables|Default|Setis_counterclockwise true))
        (else
          (Transformation|SetActorRotation (Math|Rotator|MakeRotator _roll _pitch (+ _yaw (* (Variables|Default|Getrot_speed) DeltaSeconds)))))))
    ;[1 1 1] if cam has seen player
    (if (Variables|Default|Getspotted)
      ;[1 1 1] decrement timer
      (Variables|Default|Setseen_timer (- (Variables|Default|Getseen_timer) DeltaSeconds))
      ;[1 1 1] if it's been 5 seconds since player was seen
      (if (<= (Variables|Default|Getseen_timer) 0.0)
        ;[1 1 1] game over, man
        (bind _asisometric_player_controller (Utilities|Casting|CastToIsometricPlayerController (Game|GetPlayerController 0)))
        (Default|GameOver _asisometric_player_controller)
        (else
          ;[1 1 1] set timer text
          (Rendering|SetVisibility _timer true false)
          (Rendering|Components|TextRender|SetText _timer (Utilities|Text|ToText(Float) (Variables|Default|Getseen_timer) "HalfToEven" true 1 1 1 1))
          ;[1 1 1] rotate text towards camera
          (bind _asisometric_character (Utilities|Casting|CastToIsometricCharacter (Game|Player|GetPlayerPawn 0)))
          (Transformation|SetWorldRotation (Variables|Default|Gettext%20origin) (Math|Rotator|FindLookatRotation (Transformation|GetWorldLocation (Variables|Default|GetDefaultSceneRoot)) (Transformation|GetWorldLocation (Variables|/Game/Blueprints/IsometricCharacter.IsometricCharacter_C|GetCamera _asisometric_character))) false false)))
      (else
        ;[1 1 1] determine if there's line-of-sight from light to player
        (bind _outactors (Actor|GetAllActorsOfClass "/Game/Blueprints/glass_wall.glass_wall_C"))
        (bind _returnvalue_11 (Class|KismetSystemLibrary|LineTraceMultiNEW _returnvalue_4 _returnvalue_8 "TraceTypeQuery1" false _outactors "None" true))
        (if (Math|Boolean|ANDBoolean (not _returnvalue_11) (< (Math|Vector|VectorLength (- _returnvalue_4 _returnvalue_8)) 1e+03) (< (Class|KismetMathLibrary|DegAcos (Math|Vector|DotProduct (Math|Vector|Normalize (Math|Vector|NegateVector (Math|Vector|GetUpVector (Transformation|GetActorRotation)))) (Math|Vector|Normalize (- (- (Transformation|GetActorLocation (Game|Player|GetPlayerPawn 0)) "0, 0,100.000000") (Transformation|GetWorldLocation (Variables|Default|GetDefaultSceneRoot)))))) (Variables|/Script/Engine.SpotLightComponent|GetOuterConeAngle (Variables|Default|GetSpotLight))))
          (Rendering|Components|Light|SetLightColor (Variables|Default|GetSpotLight) "(R=1.000000,G=0.000000,B=0.084041,A=1.000000)" true)
          (Rendering|Material|SetMaterial (Variables|Default|Getcone) 0 "/Game/Materials/camera_light_red.camera_light_red")
          (Variables|Default|Setspotted true)
          (Variables|Default|Setseen_timer 5.0))))))

(event EventBeginPlay
  (CallFunction|Reset))

(fn ConstructionScript
  (bind _defaultsceneroot (Variables|Default|GetDefaultSceneRoot))
  (bind _min_angle (Variables|Default|Getmin_angle))
  (bind _max_angle (Variables|Default|Getmax_angle))
  (bind _min_angle_2 (Variables|Default|Getmin_angle))
  (bind _defaultsceneroot_2 (Variables|Default|GetDefaultSceneRoot))
  (bind _defaultsceneroot_3 (Variables|Default|GetDefaultSceneRoot))
  (bind _max_angle_2 (Variables|Default|Getmax_angle))
  (bind _returnvalue (Transformation|GetWorldLocation _defaultsceneroot))
  (bind _returnvalue_2 (Transformation|GetWorldLocation _defaultsceneroot_2))
  (bind _returnvalue_3 (Math|Rotator|MakeRotator 0.0 0.0 _min_angle))
  (bind _returnvalue_4 (Transformation|GetWorldLocation _defaultsceneroot_3))
  (bind _returnvalue_5 (Math|Rotator|MakeRotator 0.0 0.0 _max_angle_2))
  (bind _returnvalue_6 (+ _max_angle _min_angle_2))
  (bind _returnvalue_7 (Math|Vector|GetForwardVector _returnvalue_3))
  (bind _returnvalue_8 (Math|Vector|GetForwardVector _returnvalue_5))
  (bind _returnvalue_9 (/ _returnvalue_6 2.0))
  (bind _returnvalue_10 (* _returnvalue_7 1e+02))
  (bind _returnvalue_11 (* _returnvalue_8 1e+02))
  (bind _returnvalue_12 (+ _returnvalue_9 1.8e+02))
  (bind _returnvalue_13 (Math|Rotator|MakeRotator 0.0 0.0 _returnvalue_12))
  (bind _returnvalue_14 (+ _returnvalue_2 _returnvalue_10))
  (bind _returnvalue_15 (+ _returnvalue_4 _returnvalue_11))
  (bind _returnvalue_16 (Math|Vector|GetForwardVector _returnvalue_13))
  (bind _returnvalue_17 (* _returnvalue_16 -1e+02))
  (bind _returnvalue_18 (+ _returnvalue _returnvalue_17))
  (Rendering|Debug|FlushPersistentDebugLines)
  (if (and (Variables|Default|Getrotating) (Variables|Default|Getpingpong))
    (if (> (Variables|Default|Getmin_angle) (Variables|Default|Getmax_angle))
      (Development|PrintString "!!! min angle > max angle !!!" true true "(R=1.000000,G=0.000000,B=0.079947,A=1.000000)" 5.0)
      (else
        (Rendering|Debug|DrawDebugLine _returnvalue_2 _returnvalue_14 "(R=1.000000,G=0.000000,B=0.000000,A=1.000000)" 6e+01 2.0)
        (Rendering|Debug|DrawDebugLine _returnvalue_4 _returnvalue_15 "(R=1.000000,G=0.000000,B=0.000000,A=1.000000)" 6e+01 2.0)
        (Rendering|Debug|DrawDebugArrow _returnvalue_14 _returnvalue_18 1e+02 "(R=0.049640,G=0.000000,B=1.000000,A=1.000000)" 6e+01 2.0)
        (Rendering|Debug|DrawDebugArrow _returnvalue_18 _returnvalue_15 1e+02 "(R=0.049707,G=0.000000,B=1.000000,A=1.000000)" 6e+01 2.0)))))

(fn Disable
  (Rendering|SetVisibility (Variables|Default|GetSpotLight) false false)
  (Rendering|Material|SetMaterial (Variables|Default|Getcone) 0 "/Game/Materials/camera_light_static.camera_light_static")
  (Variables|Default|Setwatching false))

(fn Reset
  (if (Variables|Default|Getwatching)
    (Rendering|SetVisibility (Variables|Default|Gettimer) false false)
    (Rendering|Components|Light|SetLightColor (Variables|Default|GetSpotLight) "(R=0.000000,G=1.000000,B=0.682082,A=1.000000)" true)
    (Rendering|Material|SetMaterial (Variables|Default|Getcone) 0 "/Game/Materials/camera_light.camera_light")
    (Variables|Default|Setspotted false)))