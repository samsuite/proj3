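; Dispenser that gives a collectible to the player, then goes on a one-minute cooldown.
; GiveCollectible disables it, resets the timer, adds its item to the first IsometricPlayerController's held collectibles and shows a pickup tooltip.
; Tick counts time while disabled and re-enables it after the cooldown.
; GiveCollectible does not check the Enabled flag itself, and nothing in this Blueprint calls it.
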(event EventTick
  (params (DeltaSeconds :type Float%20%28single-precision%29))
  (if (not (Variables|Default|Getenabled))
    (bind _output_get (Variables|Default|Settimer (+ (Variables|Default|Gettimer) DeltaSeconds)))
    ;[1 1 1] if it's been 1 minute we can dispense another item
    (if (> _output_get 6e+01)
      (Variables|Default|Setenabled true))))

(fn ConstructionScript)

(fn GiveCollectible
  (Variables|Default|Setenabled false)
  (Variables|Default|Settimer 0.0)
  (bind _asisometric_player_controller (Utilities|Casting|CastToIsometricPlayerController (Game|GetPlayerController 0)))
  (Utilities|Array|Add (Variables|/Game/Blueprints/IsometricPlayerController.IsometricPlayerController_C|Getheld_collectibles _asisometric_player_controller) (Variables|Default|Getrecieved_item))
  (Default|Tooltip _asisometric_player_controller (Utilities|String|Append "PICKED UP " (Variables|Default|Getrecieved_item))))