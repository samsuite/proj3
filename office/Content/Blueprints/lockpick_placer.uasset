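; Placer tool for the lockpick: lets the player click a nearby locked door to unlock it, or a nearby container to use the lockpick on it.
; While selected, Tick checks the hovered object's class and distance from the player, snaps the reticle to valid targets and sets target flags.
; Left click acts on those flags, then tells IsometricPlayerController the tool was used.
; The good and bad placement cubes stay hidden.
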(event EventBeginPlay
  ;[1 1 1] make the cubes invisible
  (|CallParentFunction)
  (Rendering|SetVisibility (Variables|Default|Getgoodcube) false false))

(event EventTick
  (params (DeltaSeconds :type Float%20%28single-precision%29))
  (bind _returnvalue (Game|Player|GetPlayerPawn 0))
  (bind _hovered_object (Variables|Default|Gethovered_object))
  (bind _reticle (Variables|Default|Getreticle))
  (bind _reticle_2 (Variables|Default|Getreticle))
  (bind _hit_point (Variables|Default|Gethit_point))
  (bind _returnvalue_2 (Utilities|GetClass _hovered_object))
  (bind _returnvalue_3 (Transformation|GetActorLocation _returnvalue))
  (bind _returnvalue_4 (- _returnvalue_3 "0, 0,98.000000"))
  (bind _returnvalue_5 (- _returnvalue_4 _hit_point))
  (bind _returnvalue_6 (Math|Vector|VectorLength _returnvalue_5))
  (bind _returnvalue_7 (< _returnvalue_6 2.5e+02))
  ;[1 1 1] if the mouse is over a door or container
  (|CallParentFunction DeltaSeconds)
  (if (Variables|Default|Getselected)
    (Rendering|SetVisibility (Variables|Default|Getbadcube) false true)
    (if (Utilities|ClassIsChildOf _returnvalue_2 "/Game/Blueprints/door.door_C")
      (bind _asdoor (Utilities|Casting|CastTodoor _hovered_object))
      (if (and (Variables|/Game/Blueprints/door.door_C|Getlocked _asdoor) _returnvalue_7)
        ;[1 1 1] change the target position a little since this is a door
        (bind _asdoor_2 (Utilities|Casting|CastTodoor (Variables|Default|Gethovered_object)))
        (Transformation|SetWorldLocation _reticle_2 (Transformation|GetWorldLocation (Variables|/Game/Blueprints/door.door_C|Gettarget_center _asdoor_2)) false true)
        (Rendering|SetVisibility _reticle_2 true false)
        (Variables|Default|Sethas_target true)
        (Variables|Default|Setcontainer_target false)
        (else
          (if (and (Utilities|ClassIsChildOf _returnvalue_2 "/Game/Blueprints/container.container_C") _returnvalue_7) :!label _label
            ;[1 1 1] this is a container
            (Transformation|SetWorldLocation _reticle (Transformation|GetActorLocation (Variables|Default|Gethovered_object)) false true)
            (Rendering|SetVisibility _reticle true false)
            (Variables|Default|Sethas_target true)
            (Variables|Default|Setcontainer_target true)
            (else
              (Variables|Default|Sethas_target false)
              (Variables|Default|Setcontainer_target false)))))
      (else
        (goto _label)))))

(event Input|MouseEvents|LeftMouseButton
  (params (Key :type Key%20Structure :default "AnyKey"))
  ;[1 1 1] if we're hovering over a door, unlock it
  (:Pressed
    (if (Variables|Default|Gethas_target)
      (if (Variables|Default|Getcontainer_target)
        ;[1 1 1] if we're hovering over a container, put a lockpick in it
        (bind _ascontainer (Utilities|Casting|CastTocontainer (Variables|Default|Gethovered_object)))
        (Default|UseItemon _ascontainer "/Game/Blueprints/lockpick.lockpick_C")
        (else
          (bind _asdoor (Utilities|Casting|CastTodoor (Variables|Default|Gethovered_object)))
          (Default|Unlock _asdoor)))
      ;[1 1 1] set as used
      (bind _asisometric_player_controller (Utilities|Casting|CastToIsometricPlayerController (Game|GetPlayerController 0)))
      (Default|UsedTool _asisometric_player_controller))))

(fn ConstructionScript
  (|CallParentFunction))