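; Placer tool Blueprint that spawns an RC car where the player left-clicks, provided the position is valid.
; The car spawns at the hit point, then its Cube component is turned to face opposite the placer's Rotation by negating forward and right while keeping up.
; It then calls UsedTool on the IsometricPlayerController to register the tool as used.
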(event EventBeginPlay
  (|CallParentFunction))

(event EventTick
  (params (DeltaSeconds :type Float%20%28single-precision%29))
  (|CallParentFunction 0.0))

(event Input|MouseEvents|LeftMouseButton
  (params (Key :type Key%20Structure :default "AnyKey"))
  (bind _rotation (Variables|Default|Getrotation))
  ;[1 1 1] place on click
  (:Pressed
    (if (Variables|Default|Getvalid_position)
      (bind _returnvalue (Game|SpawnActorfromClass "/Game/Blueprints/rc_car.rc_car_C" (Math|Conversions|ToTransform(Vector) (Variables|Default|Gethit_point)) "Undefined" 0 0))
      (Transformation|SetWorldRotation (Variables|/Game/Blueprints/rc_car.rc_car_C|GetCube _returnvalue) (Math|Rotator|MakeRotationfromAxes (Math|Vector|NegateVector (Math|Vector|GetForwardVector _rotation)) (Math|Vector|NegateVector (Math|Vector|GetRightVector _rotation)) (Math|Vector|GetUpVector _rotation)) false false)
      ;[1 1 1] set as used
      (bind _asisometric_player_controller (Utilities|Casting|CastToIsometricPlayerController (Game|GetPlayerController 0)))
      (Default|UsedTool _asisometric_player_controller))))

(fn ConstructionScript
  (|CallParentFunction))