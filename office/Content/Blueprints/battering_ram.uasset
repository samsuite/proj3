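; Battering ram actor that counts down three seconds after spawning, then rams whatever is in front of it and destroys itself.
; Tick decrements the timer and shows it on a text component rotated to face the IsometricCharacter's top-down camera.
; Ram spawns smoke and line traces a short way along the negated forward vector.
; A hit door is unlocked, cleared of its barricade and opened; cardboard boxes get smashed and laser juicers disabled.
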(event EventBeginPlay
  ;[1 1 1] start the timer
  (Variables|Default|Settimer 3.0))

(event EventTick
  (params (DeltaSeconds :type Float%20%28single-precision%29))
  (bind _timer_text (Variables|Default|Gettimer_text))
  ;[1 1 1] decrement the timer
  (bind _output_get (Variables|Default|Settimer (- (Variables|Default|Gettimer) DeltaSeconds)))
  ;[1 1 1] if timer is at zero, ram!
  (if (<= _output_get 0.0)
    (CallFunction|Ram)
    (else
      ;[1 1 1] set timer text
      (Rendering|SetVisibility _timer_text true false)
      (Rendering|Components|TextRender|SetText _timer_text (Utilities|Text|ToText(Float) (Variables|Default|Gettimer) "HalfToEven" true 1 1 1 1))
      ;[1 1 1] rotate text towards camera
      (bind _asisometric_character (Utilities|Casting|CastToIsometricCharacter (Game|Player|GetPlayerPawn 0)))
      (Transformation|SetWorldRotation (Variables|Default|Gettext%20origin) (Math|Rotator|FindLookatRotation (Transformation|GetWorldLocation (Variables|Default|GetDefaultSceneRoot)) (Transformation|GetWorldLocation (Variables|/Game/Blueprints/IsometricCharacter.IsometricCharacter_C|GetTop-Down%20Camera _asisometric_character))) false false))))

(fn ConstructionScript)

(fn Ram
  (bind _defaultsceneroot (Variables|Default|GetDefaultSceneRoot))
  (bind _returnvalue (Transformation|GetWorldLocation _defaultsceneroot))
  (bind _returnvalue_2 (+ _returnvalue "0,0.000000,10.000000"))
  (Effects|SpawnEmitteratLocation "/Game/Particles/smoke_effect.smoke_effect" (Transformation|GetWorldLocation (Variables|Default|GetDefaultSceneRoot)))
  ;[1 1 1] raycast ahead
  (bind _outhit (Collision|LineTraceByChannel _returnvalue_2 (+ _returnvalue_2 (* (Math|Vector|GetForwardVector (Transformation|GetWorldRotation _defaultsceneroot)) -1.5e+02)) "TraceTypeQuery1" false 0 "None"))
  ;[1 1 1] did we hit a door or a box?
  (if (Utilities|ClassIsChildOf (Utilities|GetClass (.HitActor (Collision|BreakHitResult _outhit))) "/Game/Blueprints/door.door_C")
    (bind _asdoor (Utilities|Casting|CastTodoor (.HitActor (Collision|BreakHitResult _outhit))))
    (Default|Unlock _asdoor)
    (Default|RemoveBarricade _asdoor)
    (Default|Open _asdoor)
    (elif (Utilities|ClassIsChildOf (Utilities|GetClass (.HitActor (Collision|BreakHitResult _outhit))) "/Game/Blueprints/cardboard_box.cardboard_box_C")
      (bind _ascardboard_box (Utilities|Casting|CastTocardboard_box (.HitActor (Collision|BreakHitResult _outhit))))
      (Default|Smash _ascardboard_box)
      (elif (Utilities|ClassIsChildOf (Utilities|GetClass (.HitActor (Collision|BreakHitResult _outhit))) "/Game/Blueprints/laser_juicer.laser_juicer_C")
        (bind _aslaser_juicer (Utilities|Casting|CastTolaser_juicer (.HitActor (Collision|BreakHitResult _outhit))))
        (Default|Disable _aslaser_juicer))))
  (Actor|DestroyActor))