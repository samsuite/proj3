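; RC car gadget that carries a held item forward until it crashes, then applies that item at the impact point.
; Using an item on it activates physics and the roll sound, and Tick drives the cube forward at constant speed while keeping vertical velocity.
; Any hit without a straight-up normal triggers smoke and destroys the car, detonating carried bombs or ink bombs.
; Struck doors are unlocked by a lockpick and open unless locked or barricaded.
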(event EventTick
  (params (DeltaSeconds :type Float%20%28single-precision%29))
  (bind _cube (Variables|Default|GetCube))
  (bind _returnvalue (Transformation|GetWorldRotation _cube))
  (bind _returnvalue_2 (Math|Vector|GetForwardVector _returnvalue))
  (bind _returnvalue_3 (* _returnvalue_2 5e+02))
  (bind (_x _y) (Math|Vector|BreakVector _returnvalue_3))
  (if (Variables|Default|Getactivated)
    (Class|PrimitiveComponent|SetAllPhysicsLinearVelocity _cube (Math|Vector|MakeVector _x _y (.Z (Math|Vector|BreakVector (Transformation|GetComponentVelocity (Variables|Default|GetCube))))) false)))

(event EventUseItemon
  (params (item :type Holdable%20Class%20Reference))
  (Variables|Default|Setheld_item item)
  (CallFunction|Activate))

(event Collision|EventHit
  (params (MyComp :type Primitive%20Component%20Object%20Reference) (Other :type Actor%20Object%20Reference) (OtherComp :type Primitive%20Component%20Object%20Reference) (bSelfMoved :type Boolean) (HitLocation :type Vector :default "0, 0, 0") (HitNormal :type Vector) (NormalImpulse :type Vector :default "0, 0, 0") (Hit :type Hit%20Result%20Structure%20%28by%20ref%29))
  (if (Variables|Default|Getactivated)
    (if (not (Math|Vector|Equal(Vector) HitNormal "0, 0,1.000000" 0.0001))
      (CallFunction|Done Other))))

(fn ConstructionScript
  (|CallParentFunction))

(fn Done
  (params (hit%20object :type Actor%20Object%20Reference))
  (bind _cube (Variables|Default|GetCube))
  (bind _returnvalue (Transformation|GetWorldLocation _cube))
  (bind _returnvalue_2 (+ _returnvalue "0, 0,50.000000"))
  (bind _returnvalue_3 (Math|Conversions|ToTransform(Vector) _returnvalue_2))
  (Audio|Components|Audio|Stop (Variables|Default|Getroll))
  (Audio|PlaySound2D "/Game/Sound/rc_car_collision_with_stuff.rc_car_collision_with_stuff")
  (Physics|SetSimulatePhysics _cube false)
  (Collision|SetCollisionEnabled _cube "NoCollision")
  (Effects|SpawnEmitteratLocation "/Game/Particles/smoke_effect.smoke_effect" _returnvalue "0.000000, 0, 0")
  (if (Utilities|ClassIsChildOf (Variables|Default|Getheld_item) "/Game/Blueprints/bomb.bomb_C")
    (bind _returnvalue_4 (Game|SpawnActorfromClass "/Game/Blueprints/bomb.bomb_C" _returnvalue_3 "Undefined" 0 0))
    (Default|Explode _returnvalue_4)
    (elif (Utilities|ClassIsChildOf (Variables|Default|Getheld_item) "/Game/Blueprints/ink_bomb.ink_bomb_C")
      (bind _returnvalue_5 (Game|SpawnActorfromClass "/Game/Blueprints/ink_bomb.ink_bomb_C" _returnvalue_3 "Undefined" 0 0))
      (Default|Explode _returnvalue_5)))
  (if (Utilities|ClassIsChildOf (Utilities|GetClass hit%20object) "/Game/Blueprints/door.door_C")
    (bind _asdoor (Utilities|Casting|CastTodoor hit%20object))
    (if (Utilities|ClassIsChildOf (Variables|Default|Getheld_item) "/Game/Blueprints/lockpick.lockpick_C")
      (Default|Unlock _asdoor))
    (if (and (not (Variables|/Game/Blueprints/door.door_C|Getlocked _asdoor)) (not (Variables|/Game/Blueprints/door.door_C|Getbarricaded _asdoor)))
      (Default|Open _asdoor)))
  (Actor|DestroyActor))

(fn Activate
  (Variables|Default|Setactivated true)
  (Physics|SetSimulatePhysics (Variables|Default|GetCube) true)
  (Audio|Components|Audio|Play (Variables|Default|Getroll) 0.0))