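; Placement tool that previews a grappling hook and spawns it on left click, linked to a Grapple_target.
; While selected at a valid position, each tick picks the target closest in horizontal angle to its reversed forward vector, within a narrow cone, range and height limit.
; The reticle marks that target; having none on the previous scan shows the bad cube.
; Placing requires a target and notifies IsometricPlayerController that the tool is used.
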(event EventBeginPlay
  (|CallParentFunction)
  ;[1 1 1] get all targetable objects
  (bind _outactors (Actor|GetAllActorsOfClass "/Game/Blueprints/grapple_target.grapple_target_C"))
  (Utilities|Array|AppendArray (Variables|Default|Getgrap_targets) _outactors))

(event EventTick
  (params (DeltaSeconds :type Float%20%28single-precision%29))
  (bind _returnvalue (Transformation|GetActorRotation))
  (bind _grap_targets (Variables|Default|Getgrap_targets))
  (bind _returnvalue_2 (Math|Vector|GetForwardVector _returnvalue))
  (bind _returnvalue_3 (Math|Vector|NegateVector _returnvalue_2))
  (bind (_x _y) (Math|Vector|BreakVector _returnvalue_3))
  (|CallParentFunction 0.0)
  (if (Variables|Default|Getselected)
    (if (Variables|Default|Getvalid_position)
      (if (== (Variables|Default|Gettarget) self)
        (Rendering|SetVisibility (Variables|Default|Getgoodcube) false false)
        (Rendering|SetVisibility (Variables|Default|Getbadcube) true false))
      ;[0.2237 0.8498 1] reset vars
      (Variables|Default|Setmin_angle 3.6e+02)
      (Variables|Default|Settarget self)
      ;[0.265 0.265 0.265] loop through all objects & look for a target
      (for _index (range 0 (- (Utilities|Array|Length _grap_targets) 1))
        (if (Math|Boolean|ANDBoolean (< (Class|KismetMathLibrary|DegAcos (Math|Vector|DotProduct (Math|Vector|Normalize (Math|Vector|MakeVector _x _y 0.0)) (Math|Vector|Normalize (Math|Vector|MakeVector (.X (Math|Vector|BreakVector (- (Transformation|GetActorLocation (Utilities|Array|Get(acopy) _grap_targets _index)) (Transformation|GetWorldLocation (Variables|Default|GetDefaultSceneRoot))))) (.Y (Math|Vector|BreakVector (- (Transformation|GetActorLocation (Utilities|Array|Get(acopy) _grap_targets _index)) (Transformation|GetWorldLocation (Variables|Default|GetDefaultSceneRoot))))) 0.0)))) (Variables|Default|Getmin_angle)) (< (Class|KismetMathLibrary|DegAcos (Math|Vector|DotProduct (Math|Vector|Normalize (Math|Vector|MakeVector _x _y 0.0)) (Math|Vector|Normalize (Math|Vector|MakeVector (.X (Math|Vector|BreakVector (- (Transformation|GetActorLocation (Utilities|Array|Get(acopy) _grap_targets _index)) (Transformation|GetWorldLocation (Variables|Default|GetDefaultSceneRoot))))) (.Y (Math|Vector|BreakVector (- (Transformation|GetActorLocation (Utilities|Array|Get(acopy) _grap_targets _index)) (Transformation|GetWorldLocation (Variables|Default|GetDefaultSceneRoot))))) 0.0)))) 2e+01) (< (Math|Vector|VectorLength (Math|Vector|MakeVector (.X (Math|Vector|BreakVector (- (Transformation|GetActorLocation (Utilities|Array|Get(acopy) _grap_targets _index)) (Transformation|GetWorldLocation (Variables|Default|GetDefaultSceneRoot))))) (.Y (Math|Vector|BreakVector (- (Transformation|GetActorLocation (Utilities|Array|Get(acopy) _grap_targets _index)) (Transformation|GetWorldLocation (Variables|Default|GetDefaultSceneRoot))))) 0.0)) 9e+02) (> (.Z (Math|Vector|BreakVector (- (Transformation|GetActorLocation (Utilities|Array|Get(acopy) _grap_targets _index)) (Transformation|GetWorldLocation (Variables|Default|GetDefaultSceneRoot))))) -1.0))
          (Variables|Default|Settarget (Utilities|Array|Get(acopy) _grap_targets _index))
          (Variables|Default|Setmin_angle (Class|KismetMathLibrary|DegAcos (Math|Vector|DotProduct (Math|Vector|Normalize (Math|Vector|MakeVector _x _y 0.0)) (Math|Vector|Normalize (Math|Vector|MakeVector (.X (Math|Vector|BreakVector (- (Transformation|GetActorLocation (Utilities|Array|Get(acopy) _grap_targets _index)) (Transformation|GetWorldLocation (Variables|Default|GetDefaultSceneRoot))))) (.Y (Math|Vector|BreakVector (- (Transformation|GetActorLocation (Utilities|Array|Get(acopy) _grap_targets _index)) (Transformation|GetWorldLocation (Variables|Default|GetDefaultSceneRoot))))) 0.0)))))))
      ;[0.6935 0.4267 1] once we have a target, mark which target it is
      (if (not (== (Variables|Default|Gettarget) self))
        (Transformation|SetWorldLocation (Variables|Default|Getreticle) (Transformation|GetActorLocation (Variables|Default|Gettarget)) false false)
        (Rendering|SetVisibility (Variables|Default|Getreticle) true false)))))

(event Input|MouseEvents|LeftMouseButton
  (params (Key :type Key%20Structure :default "AnyKey"))
  ;[1 1 1] place on click
  (:Pressed
    (if (and (Variables|Default|Getvalid_position) (!= (Variables|Default|Gettarget) self))
      (bind _returnvalue (Game|SpawnActorfromClass "/Game/Blueprints/grappling_hook.grappling_hook_C" (Math|Conversions|ToTransform(Vector) (Variables|Default|Gethit_point)) "Undefined" 0 0))
      (Transformation|SetActorRotation _returnvalue (Variables|Default|Getrotation))
      (Variables|/Game/Blueprints/grappling_hook.grappling_hook_C|Setgrap_target _returnvalue (Variables|Default|Gettarget))
      ;[1 1 1] set as used
      (bind _asisometric_player_controller (Utilities|Casting|CastToIsometricPlayerController (Game|GetPlayerController 0)))
      (Default|UsedTool _asisometric_player_controller))))

(fn ConstructionScript
  (|CallParentFunction))