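; Wall actor for an isometric view that swaps to a transparent version when it blocks the camera's view of the player.
; Each tick, a component line trace against the solid Wall runs from 98 units below the player's location to the IsometricCharacter camera.
; A hit hides Wall and shows TransparentWall, an instant visibility toggle rather than a gradual fade.
; The construction script stretches Origin along X from the Length variable.
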(event EventBeginPlay
  (Rendering|SetVisibility (Variables|Default|Gettransparent_wall) true false)
  (Collision|SetCollisionObjectType (Variables|Default|Getwall) "ECC_WorldDynamic"))

(event EventTick
  (params (DeltaSeconds :type Float%20%28single-precision%29))
  (bind _asisometric_character (Utilities|Casting|CastToIsometricCharacter (Game|Player|GetPlayerPawn 0)))
  (bind _returnvalue (Collision|LineTraceComponent (Variables|Default|Getwall) (- (Transformation|GetActorLocation (Game|Player|GetPlayerPawn 0)) "0, 0,98.000000") (Transformation|GetWorldLocation (Variables|/Game/Blueprints/IsometricCharacter.IsometricCharacter_C|GetCamera _asisometric_character)) true false))
  (Development|SetHiddeninGame (Variables|Default|Getwall) _returnvalue false)
  (Development|SetHiddeninGame (Variables|Default|Gettransparent_wall) (not _returnvalue) false))

(fn ConstructionScript
  (Transformation|SetWorldScale3D (Variables|Default|Getorigin) (Math|Vector|MakeVector (/ (Variables|Default|Getlength) 1e+02) 1.0 1.0)))