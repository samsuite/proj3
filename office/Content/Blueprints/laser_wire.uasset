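; Laser tripwire trap that starts a countdown to game over when something breaks its beam.
; The construction script traces forward and backward to surrounding geometry, placing both endpoints and stretching the beam between them.
; While watching, Tick traces between the endpoints; a hit latches Spotted, reddens the beam and shows a camera-facing timer, ending in the player controller's GameOver.
; Reset re-arms a watching laser; Disable hides and deactivates it.
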(event EventTick
  (params (DeltaSeconds :type Float%20%28single-precision%29))
  (bind _defaultsceneroot (Variables|Default|GetDefaultSceneRoot))
  (bind _timer (Variables|Default|Gettimer))
  (bind _returnvalue (Transformation|GetWorldRotation _defaultsceneroot))
  (bind _returnvalue_2 (Math|Vector|GetForwardVector _returnvalue))
  ;[1 1 1] make sure laser is on
  (if (Variables|Default|Getwatching)
    ;[1 1 1] if laser has seen player
    (if (Variables|Default|Getspotted)
      ;[1 1 1] increment timer
      (Variables|Default|Setseen_timer (- (Variables|Default|Getseen_timer) DeltaSeconds))
      ;[1 1 1] if it's been 3 seconds since player was seen
      (if (<= (Variables|Default|Getseen_timer) 0.0)
        ;[1 1 1] game over, man
        (bind _asisometric_player_controller (Utilities|Casting|CastToIsometricPlayerController (Game|GetPlayerController 0)))
        (Default|GameOver _asisometric_player_controller)
        (else
          ;[1 1 1] set timer text
          (Rendering|SetVisibility _timer true false)
          (Rendering|Components|TextRender|SetText _timer (Utilities|Text|ToText(Float) (Variables|Default|Getseen_timer) "HalfToEven" true 1 1 1 1))
          ;[1 1 1] rotate text towards camera
          (bind _asisometric_character (Utilities|Casting|CastToIsometricCharacter (Game|Player|GetPlayerPawn 0)))
          (Transformation|SetWorldRotation (Variables|Default|Gettext_origin) (Math|Rotator|FindLookatRotation (Transformation|GetWorldLocation (Variables|Default|GetDefaultSceneRoot)) (Transformation|GetWorldLocation (Variables|/Game/Blueprints/IsometricCharacter.IsometricCharacter_C|GetCamera _asisometric_character))) false false)))
      (else
        (bind _returnvalue_3 (Collision|LineTraceByChannel (+ (Transformation|GetWorldLocation (Variables|Default|Getstart_center)) _returnvalue_2) (- (Transformation|GetWorldLocation (Variables|Default|Getend_center)) _returnvalue_2) "TraceTypeQuery2" false 0 "None"))
        (if _returnvalue_3
          (Rendering|Material|SetMaterial (Variables|Default|Getbeam) 0 "/Game/Materials/laser_red.laser_red")
          (Variables|Default|Setspotted true)
          (Variables|Default|Setseen_timer 3.0))))))

(event EventBeginPlay
  (CallFunction|Reset))

(fn ConstructionScript
  (bind _defaultsceneroot (Variables|Default|GetDefaultSceneRoot))
  (bind _end_center (Variables|Default|Getend_center))
  (bind _start_center (Variables|Default|Getstart_center))
  (bind _returnvalue (Transformation|GetWorldRotation _defaultsceneroot))
  (bind _returnvalue_2 (Transformation|GetWorldLocation _end_center))
  (bind _returnvalue_3 (Transformation|GetWorldLocation _start_center))
  (bind _returnvalue_4 (Transformation|GetWorldLocation _defaultsceneroot))
  (bind _returnvalue_5 (Math|Vector|GetForwardVector _returnvalue))
  (bind _returnvalue_6 (- _returnvalue_3 _returnvalue_2))
  (bind _outhit (Collision|LineTraceByChannel _returnvalue_4 (+ _returnvalue_4 (* _returnvalue_5 10000)) "TraceTypeQuery1" false 0 "None" true "(R=1.000000,G=0.000000,B=0.000000,A=1.000000)" "(R=0.000000,G=0.000000,B=0.000000,A=0.000000)" 1.0))
  (Transformation|SetWorldLocation (Variables|Default|Getend_center) (.ImpactPoint (Collision|BreakHitResult _outhit)) false true)
  (bind _outhit_2 (Collision|LineTraceByChannel _returnvalue_4 (+ (* _returnvalue_5 -10000) _returnvalue_4) "TraceTypeQuery1" false 0 "None" true "(R=1.000000,G=0.000000,B=0.000000,A=1.000000)" "(R=0.000000,G=0.000000,B=0.000000,A=0.000000)" 1.0))
  (Transformation|SetWorldLocation (Variables|Default|Getstart_center) (.ImpactPoint (Collision|BreakHitResult _outhit_2)) false true)
  (Transformation|SetWorldScale3D (Variables|Default|Getbeam) (Math|Vector|MakeVector 0.05 0.05 (- (/ (Math|Vector|VectorLength _returnvalue_6) 1e+02) 0.01)))
  (Transformation|SetWorldLocation (Variables|Default|Getbeam) (+ (/ _returnvalue_6 2) (Transformation|GetWorldLocation _end_center)) false false))

(fn Disable
  (Rendering|SetVisibility (Variables|Default|Getbeam) false false)
  (Variables|Default|Setwatching false))

(fn Reset
  (if (Variables|Default|Getwatching)
    (Rendering|SetVisibility (Variables|Default|Gettimer) false false)
    (Rendering|Material|SetMaterial (Variables|Default|Getbeam) 0 "/Game/Materials/laser_light.laser_light")
    (Variables|Default|Setspotted false)))