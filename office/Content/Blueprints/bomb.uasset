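; Bomb actor that either counts down when placed, with timer text turned toward the player's camera, or explodes on hit when launched as a projectile.
; Explode plays sound and particles, then filters all Targetable actors by radius and a Visibility line trace, with doors traced using their TargetCenter.
; Exposed targets react by class: unlocked, unbarricaded doors open, security cameras and laser juicers are disabled, cardboard boxes smash, then the bomb destroys itself.
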(event EventInit
  ;[1 1 1] if the bomb has been placed normally, set the timer and disable physics simulation
  (if (not (Variables|Default|Getis_projectile))
    (Variables|Default|Settimer 3.0)
    (Physics|SetSimulatePhysics (Variables|Default|Getcollision) false)))

(event EventTick
  (params (DeltaSeconds :type Float%20%28single-precision%29))
  (bind _timer_text (Variables|Default|Gettimer_text))
  ;[1 1 1] if the bomb has been placed normally, decrement the timer
  (if (not (Variables|Default|Getis_projectile))
    (bind _output_get (Variables|Default|Settimer (- (Variables|Default|Gettimer) DeltaSeconds)))
    ;[1 1 1] if timer is at zero, explode!
    (if (<= _output_get 0.0)
      (CallFunction|Explode)
      (else
        ;[1 1 1] set timer text
        (Rendering|SetVisibility _timer_text true false)
        (Rendering|Components|TextRender|SetText _timer_text (Utilities|Text|ToText(Float) (Variables|Default|Gettimer) "HalfToEven" true 1 1 1 1))
        ;[1 1 1] rotate text towards camera
        (bind _asisometric_character (Utilities|Casting|CastToIsometricCharacter (Game|Player|GetPlayerPawn 0)))
        (Transformation|SetWorldRotation (Variables|Default|Gettext%20origin) (Math|Rotator|FindLookatRotation (Transformation|GetWorldLocation (Variables|Default|Getroot)) (Transformation|GetWorldLocation (Variables|/Game/Blueprints/IsometricCharacter.IsometricCharacter_C|GetTop-Down%20Camera _asisometric_character))) false false)))))

(event Collision|EventHit
  (params (MyComp :type Primitive%20Component%20Object%20Reference) (Other :type Actor%20Object%20Reference) (OtherComp :type Primitive%20Component%20Object%20Reference) (bSelfMoved :type Boolean) (HitLocation :type Vector :default "0, 0, 0") (HitNormal :type Vector :default "0, 0, 0") (NormalImpulse :type Vector :default "0, 0, 0") (Hit :type Hit%20Result%20Structure%20%28by%20ref%29))
  (if (Variables|Default|Getis_projectile)
    (CallFunction|Explode)))

(fn ConstructionScript)

(fn Explode
  (bind _collision (Variables|Default|Getcollision))
  (bind _returnvalue (Transformation|GetWorldLocation _collision))
  (Audio|PlaySound2D "/Game/Sound/explosion.explosion")
  (Effects|SpawnEmitteratLocation "/Game/Particles/projectile_impact.projectile_impact" (Transformation|GetWorldLocation (Variables|Default|Getcollision)))
  (bind _outactors (Actor|GetAllActorsOfClass "/Game/Blueprints/targetable.targetable_C"))
  (for _array_element _outactors
    (if (< (Math|Vector|VectorLength (- (Transformation|GetActorLocation _array_element) _returnvalue)) 2e+02)
      (if (Utilities|ClassIsChildOf (Utilities|GetClass _array_element) "/Game/Blueprints/door.door_C")
        (bind _asdoor (Utilities|Casting|CastTodoor _array_element))
        ;[1 1 1] and we have line-of-sight to it (door)
        (bind _returnvalue_2 (Collision|LineTraceByChannel (+ (Transformation|GetActorLocation _array_element) (Transformation|GetWorldLocation (Variables|/Game/Blueprints/door.door_C|Gettarget_center _asdoor))) _returnvalue "TraceTypeQuery1" false (Utilities|Array|MakeArray _asdoor) "None"))
        (if (not _returnvalue_2)
          ;[1 1 1] open door
          (bind _asdoor_2 (Utilities|Casting|CastTodoor _array_element :!label _label))
          (if (and (not (Variables|/Game/Blueprints/door.door_C|Getlocked _asdoor_2)) (not (Variables|/Game/Blueprints/door.door_C|Getbarricaded _asdoor_2)))
            (Default|Open _asdoor_2)))
        (else
          ;[1 1 1] and we have line-of-sight to it
          (bind _returnvalue_3 (Collision|LineTraceByChannel (Transformation|GetActorLocation _array_element) _returnvalue "TraceTypeQuery1" false _outactors "None"))
          (if (not _returnvalue_3)
            (if (not (or (Utilities|ClassIsChildOf (Utilities|GetClass _array_element) "/Game/Blueprints/Catapult.catapult_C") (== _array_element self)))
              ;[1 1 1] disable camera
              (if (Utilities|ClassIsChildOf (Utilities|GetClass _array_element) "/Game/Blueprints/security_cam.security_cam_C")
                (bind _assecurity_cam (Utilities|Casting|CastTosecurity_cam _array_element))
                (Default|Disable _assecurity_cam)
                (else
                  ;[1 1 1] disable laser
                  (if (Utilities|ClassIsChildOf (Utilities|GetClass _array_element) "/Game/Blueprints/laser_juicer.laser_juicer_C")
                    (bind _aslaser_juicer (Utilities|Casting|CastTolaser_juicer _array_element))
                    (Default|Disable _aslaser_juicer)
                    (elif (Utilities|ClassIsChildOf (Utilities|GetClass _array_element) "/Game/Blueprints/door.door_C")
                      (goto _label)
                      (else
                        ;[1 1 1] destroy box
                        (if (Utilities|ClassIsChildOf (Utilities|GetClass _array_element) "/Game/Blueprints/cardboard_box.cardboard_box_C")
                          (bind _ascardboard_box (Utilities|Casting|CastTocardboard_box _array_element))
                          (Default|Smash _ascardboard_box)))))))))))))
  (Actor|DestroyActor))