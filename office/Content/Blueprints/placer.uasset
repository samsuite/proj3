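; Placement preview tool for an isometric game that follows the cursor over WorldStatic objects while Selected.
; Each Tick it moves to the cursor hit, faces the player and turns its name label to the top-down camera.
; It shows Goodcube or Badcube based on clear line of sight, closeness to the player and a flat upward surface.
; When unselected or without a hit, it parks far below the world.
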(event EventBeginPlay
  (bind _returnvalue (Game|GetPlayerController 0))
  ;[0.96 0.3526 0.1399] enable input
  (Variables|/Script/Engine.PlayerController|SetbEnableClickEvents _returnvalue true)
  (Input|EnableInput _returnvalue)
  (Rendering|Components|TextRender|SetText (Variables|Default|Gettext) (Utilities|Text|ToText(String) (Variables|Default|Gettool_name))))

(event EventTick
  (params (DeltaSeconds :type Float%20%28single-precision%29))
  (bind _returnvalue (Game|GetPlayerController 0))
  (bind _array (Utilities|Array|MakeArray "ObjectTypeQuery1"))
  (bind _hitresult (Class|PlayerController|GetHitResultUnderCursorforObjects _returnvalue _array true))
  (bind (_bblockinghit _binitialoverlap _time _location _impactpoint _normal _impactnormal _physmat _hitactor) (Collision|BreakHitResult _hitresult))
  (Rendering|SetVisibility (Variables|Default|Getreticle) false true)
  ;[1 1 1] if the item is being used
  (if (Variables|Default|Getselected)
    ;[1 1 1] rotate text towards camera
    (bind _asisometric_character (Utilities|Casting|CastToIsometricCharacter (Game|Player|GetPlayerPawn 0)))
    (Transformation|SetWorldRotation (Variables|Default|Gettext_origin) (Math|Rotator|FindLookatRotation (Transformation|GetWorldLocation (Variables|Default|Gettext_origin)) (Transformation|GetWorldLocation (Variables|/Game/Blueprints/IsometricCharacter.IsometricCharacter_C|GetTop-Down%20Camera _asisometric_character))) false false)
    (bind _output_get (Variables|Default|Sethit_point _impactpoint))
    (Variables|Default|Sethovered_object _hitactor)
    (if (Math|Vector|Equal(Vector) _impactpoint "0, 0, 0" 0.0001)
      (Transformation|SetActorLocation "0, 0,-1000000.000000" false false :!label _label)
      (else
        (Transformation|SetActorLocation _output_get false false)
        ;[0.2102 0.4569 1] rotate towards player
        (bind _output_get_2 (Variables|Default|Setrotation (Math|Conversions|RotationFromXVector (Math|Vector|RotateVector (Math|Vector|Normalize (* (- (Transformation|GetActorLocation (Game|Player|GetPlayerPawn 0)) (Transformation|GetActorLocation)) "1.000000,1.000000, 0")) "0, 0, 0"))))
        (Transformation|SetActorRotation _output_get_2)
        ;[0.8338 1 0.2846] if player has line-of-sight to hit point
        (bind _returnvalue_2 (Class|KismetSystemLibrary|LineTraceMultiNEW (+ (Variables|Default|Gethit_point) "0, 0,100.000000") (Transformation|GetActorLocation (Game|Player|GetPlayerPawn 0)) "TraceTypeQuery1" false 0 "None" true))
        (bind _output_get_3 (Variables|Default|Setvalid_position (Math|Boolean|ANDBoolean (not _returnvalue_2) (< (Math|Vector|VectorLength (- (- (Transformation|GetActorLocation (Game|Player|GetPlayerPawn 0)) "0, 0,98.000000") (Variables|Default|Gethit_point))) 2.5e+02) (Math|Vector|Equal(Vector) _normal "0, 0,1.000000" 0.0001))))
        (Rendering|SetVisibility (Variables|Default|Getreticle) false true)
        ;[1 0.09813 0.1978] if location is valid
        (if _output_get_3
          (Rendering|SetVisibility (Variables|Default|Getgoodcube) true true)
          (Rendering|SetVisibility (Variables|Default|Getbadcube) false true)
          (else
            (Rendering|SetVisibility (Variables|Default|Getgoodcube) false true)
            (Rendering|SetVisibility (Variables|Default|Getbadcube) true true)))))
    (else
      (goto _label))))

(fn ConstructionScript
  (|CallParentFunction))