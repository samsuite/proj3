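; Catapult actor that launches a used item as a projectile, then destroys itself after the single shot.
; Using an item on it plays launch sound and smoke, spawns that class, flags it as a projectile and initializes it.
; With itself as Target, it lobs the projectile upward along negative forward.
; Otherwise it disables gravity and fires straight at the Target, aiming at TargetCenter for doors.
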(event EventBeginPlay)

(event EventUseItemon
  (params (item :type Holdable%20Class%20Reference))
  (CallFunction|Fire item))

(fn ConstructionScript)

(fn Fire
  (params (ProjectileClass :type Holdable%20Class%20Reference))
  (bind _defaultsceneroot (Variables|Default|GetDefaultSceneRoot))
  (bind _defaultsceneroot_2 (Variables|Default|GetDefaultSceneRoot))
  (bind _returnvalue (Transformation|GetWorldLocation _defaultsceneroot_2))
  (bind _returnvalue_2 (Transformation|GetWorldLocation _defaultsceneroot))
  (Audio|PlaySound2D "/Game/Sound/catapult_launch.catapult_launch")
  (Effects|SpawnEmitteratLocation "/Game/Particles/smoke_effect.smoke_effect" _returnvalue_2)
  (bind _returnvalue_3 (Game|SpawnActorfromClass ProjectileClass (Math|Conversions|ToTransform(Vector) _returnvalue_2) "AlwaysSpawn" 0 0))
  (Variables|/Game/Blueprints/holdable.holdable_C|Setis_projectile _returnvalue_3 true)
  (Default|Init _returnvalue_3)
  (if (== (Variables|Default|Gettarget) self)
    (Physics|AddImpulse (Variables|/Game/Blueprints/holdable.holdable_C|Getcollision _returnvalue_3) (+ (* (Math|Vector|GetForwardVector (Transformation|GetActorRotation)) -1500) "0,0.000000,800.000000") "None" true)
    (else
      (Physics|SetEnableGravity (Variables|/Game/Blueprints/holdable.holdable_C|Getcollision _returnvalue_3) false)
      (if (Utilities|ClassIsChildOf (Utilities|GetClass (Variables|Default|Gettarget)) "/Game/Blueprints/door.door_C")
        (bind _asdoor (Utilities|Casting|CastTodoor (Variables|Default|Gettarget)))
        (Physics|AddImpulse (Variables|/Game/Blueprints/holdable.holdable_C|Getcollision _returnvalue_3) (* (Math|Vector|Normalize (- (Transformation|GetWorldLocation (Variables|/Game/Blueprints/door.door_C|Gettarget_center _asdoor)) _returnvalue)) 2000) "None" true)
        (else
          (Physics|AddImpulse (Variables|/Game/Blueprints/holdable.holdable_C|Getcollision _returnvalue_3) (* (Math|Vector|Normalize (- (Transformation|GetActorLocation (Variables|Default|Gettarget)) _returnvalue)) 2000) "None" true)))))
  (Actor|DestroyActor))