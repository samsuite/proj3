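; Player controller for an isometric gadget game with cameras and lasers, managing held tools, HUD, crafting view and checkpointing.
; Tools are spawned placer actors; selecting one makes it current, and using one destroys it and reverts to an empty tool.
; Shift toggles an inventory built from held tools; Tab blends to a tagged crafting camera.
; GameOver destroys placed tools, resets cameras and lasers, then restores the pawn transform saved at BeginPlay.
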(event EventBeginPlay
  (Variables|Default|SetbEnableClickEvents true)
  (Variables|Default|SetbShowMouseCursor true)
  (bind _returnvalue (Game|SpawnActorfromClass "/Game/Blueprints/grabber.grabber_C" (Math|Transform|MakeTransform "0, 0, 0") "Undefined" 0 0))
  (Variables|Default|Setitem_grabber _returnvalue)
  ;[1 1 1] add HUD
  (bind _returnvalue_2 (UserInterface|CreateWidget "/Game/Blueprints/hud.hud_C"))
  (bind _output_get (Variables|Default|Sethud_reference _returnvalue_2))
  (UserInterface|Viewport|AddtoViewport _output_get 0)
  ;[1 1 1] create empty tool and set it as the current tool
  (bind _returnvalue_3 (Game|SpawnActorfromClass "/Game/Blueprints/no_tool.no_tool_C" (Math|Transform|MakeTransform "0,0.000000, 0" "0.000000, 0, 0") "Undefined" 0 0))
  (bind _output_get_2 (Variables|Default|Setnone_tool _returnvalue_3))
  (bind _output_get_3 (Variables|Default|Setcurrent_tool _output_get_2))
  (CallFunction|SelectTool _output_get_3)
  (Utilities|Array|Add (Variables|Default|Getheld_tools) _returnvalue_3)
  (CallFunction|SaveGame)
  ;[1 1 1] give ourselves some stuff to play with
  (CallFunction|GiveTool "/Game/Blueprints/catapult_placer.catapult_placer_C")
  (CallFunction|GiveTool "/Game/Blueprints/bomb_placer.bomb_placer_C")
  (CallFunction|GiveTool "/Game/Blueprints/lockpick_placer.lockpick_placer_C")
  (CallFunction|GiveTool "/Game/Blueprints/ink_bomb_placer.ink_bomb_placer_C")
  (CallFunction|GiveTool "/Game/Blueprints/ink_bomb_placer.ink_bomb_placer_C")
  (CallFunction|GiveTool "/Game/Blueprints/lockpick_placer.lockpick_placer_C")
  (CallFunction|GiveTool "/Game/Blueprints/grapple_placer.grapple_placer_C")
  (CallFunction|GiveTool "/Game/Blueprints/bomb_placer.bomb_placer_C")
  (CallFunction|GiveTool "/Game/Blueprints/ram_placer.ram_placer_C")
  (CallFunction|GiveTool "/Game/Blueprints/ram_placer.ram_placer_C")
  (CallFunction|GiveTool "/Game/Blueprints/ram_placer.ram_placer_C"))

(event Input|KeyboardEvents|LeftShift
  (params (Key :type Key%20Structure :default "AnyKey"))
  (:Pressed
    (if (Variables|Default|Getinv_up)
      (CallFunction|HideInventory)
      (else
        (CallFunction|ShowInventory)))))

(event Input|KeyboardEvents|Tab
  (params (Key :type Key%20Structure :default "AnyKey"))
  (:Pressed
    (if (Variables|Default|Getin_crafting)
      (CallFunction|CloseCrafting)
      (else
        (CallFunction|OpenCrafting)))))

(fn ConstructionScript)

(fn GameOver
  (bind _all_placed_tools (Variables|Default|Getall_placed_tools))
  (Utilities|Array|Clear (Variables|Default|Getall_placed_tools))
  ;[1 1 1] get all placed tools
  (bind _outactors (Actor|GetAllActorsOfClass "/Game/Blueprints/bomb.bomb_C"))
  (Utilities|Array|AppendArray _all_placed_tools _outactors)
  (bind _outactors_2 (Actor|GetAllActorsOfClass "/Game/Blueprints/grappling_hook.grappling_hook_C"))
  (Utilities|Array|AppendArray _all_placed_tools _outactors_2)
  (bind _outactors_3 (Actor|GetAllActorsOfClass "/Game/Blueprints/ink_bomb.ink_bomb_C"))
  (Utilities|Array|AppendArray _all_placed_tools _outactors_3)
  (bind _outactors_4 (Actor|GetAllActorsOfClass "/Game/Blueprints/Catapult.catapult_C"))
  (Utilities|Array|AppendArray _all_placed_tools _outactors_4)
  (bind _outactors_5 (Actor|GetAllActorsOfClass "/Game/Blueprints/lockpick.lockpick_C"))
  (Utilities|Array|AppendArray _all_placed_tools _outactors_5)
  (bind _outactors_6 (Actor|GetAllActorsOfClass "/Game/Blueprints/rc_car.rc_car_C"))
  (Utilities|Array|AppendArray _all_placed_tools _outactors_6)
  (bind _outactors_7 (Actor|GetAllActorsOfClass "/Game/Blueprints/battering_ram.battering_ram_C"))
  (Utilities|Array|AppendArray _all_placed_tools _outactors_7)
  ;[1 1 1] destroy all of em
  (for _array_element (Variables|Default|Getall_placed_tools)
    (Actor|DestroyActor _array_element))
  ;[1 1 1] reset cams and lasers
  (bind _outactors_8 (Actor|GetAllActorsOfClass "/Game/Blueprints/security_cam.security_cam_C"))
  (for _array_element_2 _outactors_8
    (bind _assecurity_cam (Utilities|Casting|CastTosecurity_cam _array_element_2))
    (Default|Reset _assecurity_cam))
  (bind _outactors_9 (Actor|GetAllActorsOfClass "/Game/Blueprints/laser_wire.laser_wire_C"))
  (for _array_element_3 _outactors_9
    (bind _aslaser_wire (Utilities|Casting|CastTolaser_wire _array_element_3))
    (Default|Reset _aslaser_wire))
  (CallFunction|LoadGame))

(fn ShowInventory
  ;[1 1 1] make hud visible
  (Variables|Default|Setinv_up true)
  (Widget|SetVisibility (Variables|/Game/Blueprints/hud.hud_C|Getinv (Variables|Default|Gethud_reference)) "Visible")
  ;[1 1 1] set input to UI
  (Input|SetInputModeGameandUI self (Variables|Default|Gethud_reference) "DoNotLock" true)
  ;[1 1 1] loop through held tools and make a button for each one
  (for _array_element (Variables|Default|Getheld_tools)
    (bind _returnvalue (UserInterface|CreateWidget "/Game/Blueprints/tool_element.tool_element_C"))
    (Variables|/Game/Blueprints/tool_element.tool_element_C|Setthis_tool _returnvalue _array_element)
    (Rendering|Components|TextRender|SetText (Variables|/Game/Blueprints/tool_element.tool_element_C|Getname_text _returnvalue) (Utilities|Text|ToText(String) (Variables|/Game/Blueprints/tool.tool_C|Gettool_name _array_element)))
    (Widget|Panel|AddChild (Variables|/Game/Blueprints/hud.hud_C|Gettool_list (Variables|Default|Gethud_reference)) _returnvalue)))

(fn HideInventory
  ;[1 1 1] make hud invisible
  (Variables|Default|Setinv_up false)
  (Widget|SetVisibility (Variables|/Game/Blueprints/hud.hud_C|Getinv (Variables|Default|Gethud_reference)) "Hidden")
  ;[1 1 1] erase all inventory slots
  (Widget|Panel|ClearChildren (Variables|/Game/Blueprints/hud.hud_C|Gettool_list (Variables|Default|Gethud_reference)))
  (Input|SetInputModeGameandUI self (Variables|Default|Gethud_reference) "DoNotLock" false))

(fn SelectTool
  (params (new_tool :type Tool%20Object%20Reference))
  ;[1 1 1] deselect old tool
  (Variables|/Game/Blueprints/tool.tool_C|Setselected (Variables|Default|Getcurrent_tool) false)
  ;[1 1 1] select new tool
  (Variables|/Game/Blueprints/tool.tool_C|Setselected new_tool true)
  ;[1 1 1] set new tool as current
  (Variables|Default|Setcurrent_tool new_tool)
  (CallFunction|HideInventory))

(fn UsedTool
  (bind _none_tool (Variables|Default|Getnone_tool))
  (Utilities|Array|RemoveItem (Variables|Default|Getheld_tools) (Variables|Default|Getcurrent_tool))
  (Actor|DestroyActor (Variables|Default|Getcurrent_tool))
  (Variables|Default|Setcurrent_tool _none_tool)
  (CallFunction|SelectTool _none_tool))

(fn GiveTool
  (params (tool_class :type Tool%20Class%20Reference))
  (bind _returnvalue (Game|SpawnActorfromClass tool_class (Math|Transform|MakeTransform "0,0.000000,-1000.000000" "0.000000, 0, 0") "AlwaysSpawn" 0 0))
  (Utilities|Array|Add (Variables|Default|Getheld_tools) _returnvalue))

(fn SaveGame
  (bind _returnvalue (SaveGame|CreateSaveGameObject "/Game/Blueprints/save_obj.save_obj_C"))
  (bind _assave_obj (Utilities|Casting|CastTosave_obj _returnvalue))
  (Variables|Default|Setsave_instance _assave_obj)
  ;[1 1 1] save player location
  (Variables|/Game/Blueprints/save_obj.save_obj_C|Setplayer_location (Variables|Default|Getsave_instance) (Transformation|GetActorLocation (Game|Player|GetPlayerPawn 0)))
  ;[1 1 1] save player rotation
  (Variables|/Game/Blueprints/save_obj.save_obj_C|Setplayer_rotation (Variables|Default|Getsave_instance) (Transformation|GetActorRotation (Game|Player|GetPlayerPawn 0)))
  (SaveGame|SaveGametoSlot (Variables|Default|Getsave_instance) "slot0"))

(fn LoadGame
  ;[1 1 1] if there's anything to load
  (bind _returnvalue (SaveGame|DoesSaveGameExist "slot0"))
  (if _returnvalue
    (bind _returnvalue_2 (SaveGame|LoadGamefromSlot "slot0"))
    (bind _assave_obj (Utilities|Casting|CastTosave_obj _returnvalue_2))
    (Variables|Default|Setsave_instance _assave_obj)
    ;[1 1 1] load player location
    (Transformation|SetActorLocation (Game|Player|GetPlayerPawn 0) (Variables|/Game/Blueprints/save_obj.save_obj_C|Getplayer_location (Variables|Default|Getsave_instance)) false true)
    ;[1 1 1] load player rotation
    (Transformation|SetActorRotation (Game|Player|GetPlayerPawn 0) (Variables|/Game/Blueprints/save_obj.save_obj_C|Getplayer_rotation (Variables|Default|Getsave_instance)))))

(fn Tooltip
  (params (text :type String))
  (Widget|SetVisibility (Variables|/Game/Blueprints/hud.hud_C|Getgot_item (Variables|Default|Gethud_reference)) "HitTestInvisible")
  (Rendering|Components|TextRender|SetText (Variables|/Game/Blueprints/hud.hud_C|Getitem_text (Variables|Default|Gethud_reference)) (Utilities|Text|ToText(String) text))
  (Variables|/Game/Blueprints/hud.hud_C|Setitem_timer (Variables|Default|Gethud_reference) 1.0))

(fn OpenCrafting
  (Variables|Default|Setin_crafting true)
  (bind _outactors (Actor|GetAllActorswithTag "CraftingCamera"))
  (Game|Player|SetViewTargetwithBlend (Utilities|Array|Get(acopy) _outactors) 0.0 "VTBlend_Linear" 0.0 false))

(fn CloseCrafting
  (Variables|Default|Setin_crafting false)
  (bind _asisometric_character (Utilities|Casting|CastToIsometricCharacter (Game|Player|GetPlayerPawn 0)))
  (Game|Player|SetViewTargetwithBlend _asisometric_character 0.0 "VTBlend_Linear" 0.0 false))