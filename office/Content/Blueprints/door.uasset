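; Interactive hinged door that the player opens and closes with E when within range and nearest, unless it is locked or barricaded.
; Every Tick, each door scans all doors for the closest, shows a state prompt turned toward the isometric camera, and interpolates its hinge toward open or closed rotations.
; Functions set the open state and clear locks or barricades, while the construction script draws debug orientation arrows.
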(event EventBeginPlay
  ;[1 1 1] enable input
  (Input|EnableInput (Game|GetPlayerController 0))
  (Collision|SetCollisionObjectType (Variables|Default|Getcollision) "ECC_WorldStatic"))

(event EventTick
  (params (DeltaSeconds :type Float%20%28single-precision%29))
  (bind _defaultsceneroot (Variables|Default|GetDefaultSceneRoot))
  (bind _outactors (Actor|GetAllActorsOfClass "door_C"))
  (Variables|Default|Setmin_dist 99999.0)
  (for _array_element _outactors
    (if (< (Math|Vector|VectorLength (- (Transformation|GetActorLocation (Game|Player|GetPlayerPawn 0)) (+ (Transformation|GetWorldLocation (Variables|/Game/Blueprints/targetable.targetable_C|GetDefaultSceneRoot _array_element)) (* (Math|Vector|GetForwardVector (Transformation|GetWorldRotation (Variables|/Game/Blueprints/targetable.targetable_C|GetDefaultSceneRoot _array_element))) -50)))) (Variables|Default|Getmin_dist))
      (Variables|Default|Setmin_dist (Math|Vector|VectorLength (- (Transformation|GetActorLocation (Game|Player|GetPlayerPawn 0)) (+ (Transformation|GetWorldLocation (Variables|/Game/Blueprints/targetable.targetable_C|GetDefaultSceneRoot _array_element)) (* (Math|Vector|GetForwardVector (Transformation|GetWorldRotation (Variables|/Game/Blueprints/targetable.targetable_C|GetDefaultSceneRoot _array_element))) -50)))))
      (Variables|Default|Setmin_door _array_element)))
  (Rendering|SetVisibility (Variables|Default|Gettext) (and (< (Math|Vector|VectorLength (- (Transformation|GetActorLocation (Game|Player|GetPlayerPawn 0)) (+ (Transformation|GetWorldLocation _defaultsceneroot) (* (Math|Vector|GetForwardVector (Transformation|GetWorldRotation _defaultsceneroot)) -50)))) 2.5e+02) (== (Variables|Default|Getmin_door) self)) false)
  ;[1 1 1] rotate text towards camera
  (bind _asisometric_character (Utilities|Casting|CastToIsometricCharacter (Game|Player|GetPlayerPawn 0)))
  (Transformation|SetWorldRotation (Variables|Default|Gettext%20origin) (Math|Rotator|FindLookatRotation (Transformation|GetWorldLocation (Variables|Default|Gettext%20origin)) (Transformation|GetWorldLocation (Variables|/Game/Blueprints/IsometricCharacter.IsometricCharacter_C|GetTop-Down%20Camera _asisometric_character))) false false)
  ;[1 1 1] rotate the door open
  (if (Variables|Default|Getopening)
    (Rendering|Components|TextRender|SetText (Variables|Default|Gettext) (Utilities|Text|ToText(String) "[E] CLOSE"))
    (Transformation|SetWorldRotation (Variables|Default|Gethinge) (Class|KismetMathLibrary|RInterptoConstant (Transformation|GetWorldRotation (Variables|Default|Gethinge)) (Transformation|GetWorldRotation (Variables|Default|Getopened)) DeltaSeconds 3e+02) false false)
    (else
      ;[1 1 1] rotate the door closed
      (if (Variables|Default|Getclosing)
        (Rendering|Components|TextRender|SetText (Variables|Default|Gettext) (Utilities|Text|ToText(String) "[E] OPEN"))
        (Transformation|SetWorldRotation (Variables|Default|Gethinge) (Class|KismetMathLibrary|RInterptoConstant (Transformation|GetWorldRotation (Variables|Default|Gethinge)) (Transformation|GetWorldRotation (Variables|Default|Getclosed)) DeltaSeconds 3e+02) false false)
        ;[1 1 1] set locked text
        (if (Variables|Default|Getlocked)
          (Rendering|Components|TextRender|SetText (Variables|Default|Gettext) (Utilities|Text|ToText(String) "LOCKED"))
          (else
            ;[1 1 1] set barricaded text
            (if (Variables|Default|Getbarricaded)
              (Rendering|Components|TextRender|SetText (Variables|Default|Gettext) (Utilities|Text|ToText(String) "ARMORED")))))))))

(event Input|KeyboardEvents|E
  (params (Key :type Key%20Structure :default "AnyKey"))
  (bind _defaultsceneroot (Variables|Default|GetDefaultSceneRoot))
  ;[1 1 1] open or close the door when we press e
  (:Pressed
    (if (Math|Boolean|ANDBoolean (< (Math|Vector|VectorLength (- (Transformation|GetActorLocation (Game|Player|GetPlayerPawn 0)) (+ (Transformation|GetWorldLocation _defaultsceneroot) (* (Math|Vector|GetForwardVector (Transformation|GetWorldRotation _defaultsceneroot)) -50)))) 2.5e+02) (not (Variables|Default|Getlocked)) (not (Variables|Default|Getbarricaded)) (== (Variables|Default|Getmin_door) self))
      (if (Variables|Default|Getopening)
        (CallFunction|Close)
        (elif (Variables|Default|Getclosing)
          (CallFunction|Open))))))

(fn ConstructionScript
  (bind _defaultsceneroot (Variables|Default|GetDefaultSceneRoot))
  (bind _defaultsceneroot_2 (Variables|Default|GetDefaultSceneRoot))
  (bind _returnvalue (Transformation|GetWorldLocation _defaultsceneroot_2))
  (bind _returnvalue_2 (Transformation|GetWorldLocation _defaultsceneroot))
  (bind _returnvalue_3 (Transformation|GetWorldRotation _defaultsceneroot))
  (bind _returnvalue_4 (Transformation|GetWorldRotation _defaultsceneroot_2))
  (bind _returnvalue_5 (Math|Vector|GetRightVector _returnvalue_4))
  (bind _returnvalue_6 (Math|Vector|GetForwardVector _returnvalue_3))
  (bind _returnvalue_7 (Math|Vector|GetForwardVector _returnvalue_4))
  (bind _returnvalue_8 (+ _returnvalue "0.000000,0.000000,50.000000"))
  (bind _returnvalue_9 (+ _returnvalue_2 "0.000000, 0,50.000000"))
  (bind _returnvalue_10 (* _returnvalue_6 -1e+02))
  (bind _returnvalue_11 (* _returnvalue_7 -1e+02))
  (Rendering|Debug|FlushPersistentDebugLines)
  (Rendering|Debug|DrawDebugArrow (+ _returnvalue_9 _returnvalue_10) (+ (+ _returnvalue_9 (* (Math|Vector|GetRightVector _returnvalue_3) 1e+02)) _returnvalue_10) 1e+02 "(R=1.000000,G=0.000000,B=0.037428,A=1.000000)" 3e+02 1.0)
  (Rendering|Debug|DrawDebugArrow (+ (+ _returnvalue_8 (* _returnvalue_5 -1e+02)) _returnvalue_11) (+ (+ _returnvalue_8 (* _returnvalue_5 -2e+01)) _returnvalue_11) 1e+02 "(R=1.000000,G=0.000000,B=0.037428,A=1.000000)" 1e+03 1.0))

(fn Open
  (Variables|Default|Setopening true)
  (Variables|Default|Setclosing false))

(fn Close
  (Variables|Default|Setopening false)
  (Variables|Default|Setclosing true))

(fn Unlock
  (Variables|Default|Setlocked false))

(fn RemoveBarricade
  (Variables|Default|Setbarricaded false))