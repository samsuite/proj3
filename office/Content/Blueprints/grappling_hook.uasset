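; Grappling hook actor that pulls player 0's pawn toward GrapTarget and destroys itself once the pawn is within a short range.
; Each tick it snaps the Hook to the target and moves the pawn with VInterpTo and teleport, without sweep.
; The rope is faked by placing RopeRoot at the pawn-target midpoint, rotating it along that line and scaling Rope's Z by the distance.
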(event EventTick
  (params (DeltaSeconds :type Float%20%28single-precision%29))
  (bind _returnvalue (Game|Player|GetPlayerPawn 0))
  (bind _grap_target (Variables|Default|Getgrap_target))
  (bind _grap_target_2 (Variables|Default|Getgrap_target))
  (bind _returnvalue_2 (Transformation|GetActorLocation _grap_target))
  (bind _returnvalue_3 (Transformation|GetActorLocation _returnvalue))
  (bind _returnvalue_4 (Transformation|GetActorLocation _grap_target_2))
  (bind _returnvalue_5 (- _returnvalue_3 _returnvalue_4))
  (if (> (Math|Vector|VectorLength (- (Transformation|GetActorLocation (Game|Player|GetPlayerPawn 0)) _returnvalue_2)) 8e+01)
    (Transformation|SetWorldLocation (Variables|Default|Gethook) _returnvalue_2 false false)
    (Transformation|SetActorLocation _returnvalue (Math|Interpolation|VInterpTo _returnvalue_3 _returnvalue_4 DeltaSeconds 7.0) false true)
    (Transformation|SetWorldScale3D (Variables|Default|Getrope) (Math|Vector|MakeVector 0.1 0.1 (/ (Math|Vector|VectorLength _returnvalue_5) 1e+02)))
    (Transformation|SetWorldLocationAndRotation (Variables|Default|Getrope%20root) (+ (/ _returnvalue_5 2) _returnvalue_4) (Math|Rotator|FindLookatRotation _returnvalue_3 _returnvalue_4) false false)
    (else
      (Actor|DestroyActor))))

(fn ConstructionScript)