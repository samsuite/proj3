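; Ink bomb actor that works either as a projectile exploding on hit or as a placed bomb on a short fuse.
; When placed, it turns off physics and counts down on Tick, showing the timer as text turned toward the isometric character's camera.
; Explode spawns an ink impact effect, disables security cameras within range that have an unblocked visibility trace to the bomb, then destroys the actor.
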(event EventInit
  ;[1 1 1] if the bomb has been placed normally, set the timer and disable physics simulation
  (if (not (Variables|Default|Getis_projectile))
    (Variables|Default|Settimer 1.0)
    (Physics|SetSimulatePhysics (Variables|Default|Getcollision) false)))

(event EventTick
  (params (DeltaSeconds :type Float%20%28single-precision%29))
  (bind _timer_text (Variables|Default|Gettimer_text))
  ;[1 1 1] if the bomb has been placed normally, decrement the timer
  (if (not (Variables|Default|Getis_projectile))
    (bind _output_get (Variables|Default|Settimer (- (Variables|Default|Gettimer) DeltaSeconds)))
    ;[1 1 1] if timer is at zero, explode!
    (if (<= _output_get 0.0)
      (CallFunction|Explode)
      (else
        ;[1 1 1] set timer text
        (Rendering|SetVisibility _timer_text true false)
        (Rendering|Components|TextRender|SetText _timer_text (Utilities|Text|ToText(Float) (Variables|Default|Gettimer) "HalfToEven" true 1 1 1 1))
        ;[1 1 1] rotate text towards camera
        (bind _asisometric_character (Utilities|Casting|CastToIsometricCharacter (Game|Player|GetPlayerPawn 0)))
        (Transformation|SetWorldRotation (Variables|Default|Gettext%20origin) (Math|Rotator|FindLookatRotation (Transformation|GetWorldLocation (Variables|Default|Getroot)) (Transformation|GetWorldLocation (Variables|/Game/Blueprints/IsometricCharacter.IsometricCharacter_C|GetCamera _asisometric_character))) false false)))))

(event Collision|EventHit
  (params (MyComp :type Primitive%20Component%20Object%20Reference) (Other :type Actor%20Object%20Reference) (OtherComp :type Primitive%20Component%20Object%20Reference) (bSelfMoved :type Boolean) (HitLocation :type Vector :default "0, 0, 0") (HitNormal :type Vector :default "0, 0, 0") (NormalImpulse :type Vector :default "0, 0, 0") (Hit :type Hit%20Result%20Structure%20%28by%20ref%29))
  (if (Variables|Default|Getis_projectile)
    (CallFunction|Explode)))

(fn ConstructionScript)

(fn Explode
  (bind _collision (Variables|Default|Getcollision))
  (bind _returnvalue (Transformation|GetWorldLocation _collision))
  (Effects|SpawnEmitteratLocation "/Game/Particles/ink_impact.ink_impact" (Transformation|GetWorldLocation (Variables|Default|Getcollision)))
  (bind _outactors (Actor|GetAllActorsOfClass "/Game/Blueprints/security_cam.security_cam_C"))
  (for _array_element _outactors
    (if (< (Math|Vector|VectorLength (- (Transformation|GetActorLocation _array_element) _returnvalue)) 5e+02)
      ;[1 1 1] and we have line-of-sight to it
      (bind _returnvalue_2 (Collision|LineTraceByChannel (Transformation|GetActorLocation _array_element) _returnvalue "TraceTypeQuery1" false _outactors "None"))
      (if (not _returnvalue_2)
        ;[1 1 1] disable camera
        (bind _assecurity_cam (Utilities|Casting|CastTosecurity_cam _array_element))
        (Default|Disable _assecurity_cam))))
  (Actor|DestroyActor))