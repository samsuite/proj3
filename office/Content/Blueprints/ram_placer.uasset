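; Placer Blueprint that puts a battering ram into the world when the player left-clicks.
; If ValidPosition is set, it spawns a Battering_ram at HitPoint and applies the stored Rotation.
; It then calls UsedTool on the IsometricPlayerController to mark the tool as used.
; The graph only reads the position, validity and rotation values, and the construction script just runs its parent's.
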(event Input|MouseEvents|LeftMouseButton
  (params (Key :type Key%20Structure :default "AnyKey"))
  ;[1 1 1] place on click
  (:Pressed
    (if (Variables|Default|Getvalid_position)
      (bind _returnvalue (Game|SpawnActorfromClass "/Game/Blueprints/battering_ram.battering_ram_C" (Math|Conversions|ToTransform(Vector) (Variables|Default|Gethit_point)) "Undefined" 0 0))
      (Transformation|SetActorRotation _returnvalue (Variables|Default|Getrotation))
      ;[1 1 1] set as used
      (bind _asisometric_player_controller (Utilities|Casting|CastToIsometricPlayerController (Game|GetPlayerController 0)))
      (Default|UsedTool _asisometric_player_controller))))

(fn ConstructionScript
  (|CallParentFunction))